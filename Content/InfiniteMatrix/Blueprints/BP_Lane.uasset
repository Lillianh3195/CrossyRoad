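; BP_Lane is a lane actor that periodically spawns vehicles and extends the level when the chicken reaches it.
; A per-frame countdown, logged to screen, spawns a BP_Vehicle at a fixed transform when it runs out, then resets to its default.
; When BP_Chicken overlaps TriggerZone, the lane asks LaneSpawner to spawn a lane at its spawn point and destroys itself.
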(event OnComponentBeginOverlap(TriggerZone)
  (params (OverlappedComponent :type Primitive%20Component%20Object%20Reference) (OtherActor :type Actor%20Object%20Reference) (OtherComp :type Primitive%20Component%20Object%20Reference) (OtherBodyIndex :type Integer) (bFromSweep :type Boolean) (SweepResult :type Hit%20Result%20Structure%20%28by%20ref%29))
  (Utilities|Casting|CastToBP_Chicken OtherActor)
  (Default|SpawnLaneatSpawnPoint (Variables|Default|GetLaneSpawner))
  (Actor|DestroyActor))

(event EventBeginPlay
  (bind _output_get (Variables|Default|SetCountdown (Variables|Default|GetDefaultCountdown)))
  (Development|PrintString (Utilities|String|ToString(Integer) _output_get) true true "(R=0.000000,G=0.660000,B=1.000000,A=1.000000)" 5.0)
  (if (<= (stale EventTick _output_get) 0)
    (Game|SpawnActorfromClass "/Game/InfiniteMatrix/Blueprints/BP_Vehicle.BP_Vehicle_C" (Math|Transform|MakeTransform "0.000000,0.000000,-10.000000" "0, 0, 0" "1.000000,1.000000,1.000000") "Undefined" "MultiplyWithRoot" self 0)
    (Variables|Default|SetCountdown (Variables|Default|GetDefaultCountdown))
    (Development|PrintString "Spawned a Car" true true "(R=0.000000,G=0.660000,B=1.000000,A=1.000000)" 5.0)))

(event EventTick
  (params (DeltaSeconds :type Float%20%28single-precision%29))
  (bind _result (Math|Integer|DecrementInt (Variables|Default|GetCountdown))
    (:%20%20
      (bind _output_get (Variables|Default|SetCountdown _result))
      (Development|PrintString (Utilities|String|ToString(Integer) (stale EventBeginPlay _output_get)) true true "(R=0.000000,G=0.660000,B=1.000000,A=1.000000)" 5.0)
      (if (<= _output_get 0)
        (Game|SpawnActorfromClass "/Game/InfiniteMatrix/Blueprints/BP_Vehicle.BP_Vehicle_C" (Math|Transform|MakeTransform "0.000000,0.000000,-10.000000" "0, 0, 0" "1.000000,1.000000,1.000000") "Undefined" "MultiplyWithRoot" self 0)
        (Variables|Default|SetCountdown (Variables|Default|GetDefaultCountdown))
        (Development|PrintString "Spawned a Car" true true "(R=0.000000,G=0.660000,B=1.000000,A=1.000000)" 5.0)))))

(fn ConstructionScript)