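; BP_LaneSpawner builds a starting strip of random grass, highway, river and train track lanes, beginning at the player pawn.
; On BeginPlay it destroys existing BP_Lanes, then chains new ones from each newest lane's SpawnPoint.
; SpawnRandomLaneType re-rolls to avoid repeating the last type, spawns one or two lanes, and leaves a group's final highway unmarked.
; Each lane gets a reference back to the spawner; vehicle spawning is unconnected.
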(event EventBeginPlay
  (CallFunction|SpawnInitialLanes)
  (Development|PrintString "Initial Lanes Spawned"))

(event Collision|EventActorBeginOverlap
  (params (OtherActor :type Actor%20Object%20Reference)))

(event EventTick
  (params (DeltaSeconds :type Float%20%28single-precision%29)))

(fn ConstructionScript)

(fn SpawnLane
  (params (SpawnLocation :type Vector) (StaticMesh :type Static%20Mesh%20Object%20Reference))
  (bind _returnvalue (Game|SpawnActorfromClass "/Game/InfiniteMatrix/Blueprints/BP_Lane.BP_Lane_C" (Math|Transform|MakeTransform SpawnLocation "0, 0, 0" "1.000000,1.000000,1.000000") "Undefined" "MultiplyWithRoot" 0 0))
  (Components|StaticMesh|SetStaticMesh (Variables|/Game/InfiniteMatrix/Blueprints/BP_Lane.BP_Lane_C|GetLane _returnvalue) StaticMesh)
  (bind _output_get (Variables|Default|SetNewestLane _returnvalue))
  (Variables|/Game/InfiniteMatrix/Blueprints/BP_Lane.BP_Lane_C|SetLaneSpawner _output_get self)
  (bind _result (Math|Integer|IncrementInt (Variables|Default|GetlanesSpawned))
    (:%20%20
      (bind _output_get_2 (Variables|Default|SetlanesSpawned _result))
      (Development|PrintString (Utilities|String|ToString(Text) (Utilities|Text|FormatText "\"                  Lanes spawned:    {N} at {x}\"" _output_get_2 (.X (Math|Vector2D|BreakVector2D (Math|Conversions|ToVector2D(Vector) SpawnLocation))))) true true "(R=1.000000,G=0.026376,B=0.191370,A=1.000000)" 5.0))))

(fn SpawnLaneatSpawnPoint
  (CallFunction|SpawnRandomLaneType self (Transformation|GetWorldLocation (Variables|/Game/InfiniteMatrix/Blueprints/BP_Lane.BP_Lane_C|GetSpawnPoint (Variables|Default|GetNewestLane)))))

(fn SpawnInitialLanes
  (Utilities|FlowControl|Sequence
    (:then_0
      (bind _outactors (Actor|GetAllActorsOfClass "/Game/InfiniteMatrix/Blueprints/BP_Lane.BP_Lane_C"))
      (for _array_element _outactors
        (Actor|DestroyActor _array_element)))
    (:then_1
      (for _index (range 0 8)
        (Utilities|IsValid (Variables|Default|GetNewestLane)
          (:Is%20Valid
            (CallFunction|SpawnLaneatSpawnPoint))
          (:Is%20Not%20Valid
            (CallFunction|SpawnRandomLaneType (Transformation|GetActorLocation (Game|Player|GetPlayerPawn 0)))))))))

(fn SpawnRandomLaneType
  (params (SpawnLocation :type Vector))
  (bind _returnvalue (Math|Random|RandomIntegerinRange 1 2))
  (bind _newestlane (Variables|Default|GetNewestLane))
  (LocalVariables|Setnew%20Location SpawnLocation)
  (bind _output_get (Variables|Default|SetmeshTypeIndex (Math|Random|RandomIntegerinRange 0 3) :!label _label))
  (if (== _output_get (Variables|Default|GetlastMeshTypeIndex))
    (goto _label)
    (else
      (Variables|Default|SetlastMeshTypeIndex (Variables|Default|GetmeshTypeIndex))
      (Variables|Default|SetmaxLanes _returnvalue)
      (Development|PrintString (Utilities|String|ToString(Text) (Utilities|Text|FormatText "\"Spawning {N} lanes of type {mesh}\"" _returnvalue (Variables|Default|GetmeshTypeIndex))) true true "(R=0.000000,G=0.660000,B=1.000000,A=1.000000)" 2e+01)
      (for _index (range 1 (Variables|Default|GetmaxLanes))
        (LocalVariables|SetnewMesh (Utilities|Select :Index (Variables|Default|GetmeshTypeIndex) :Option%200 "/Game/InfiniteMatrix/Meshes/SM_grass.SM_grass" :Option%201 "/Game/InfiniteMatrix/Meshes/SM_highway1_marked.SM_highway1_marked" :Option%202 "/Game/InfiniteMatrix/Meshes/SM_river1.SM_river1" :Option%203 "/Game/InfiniteMatrix/Meshes/SM_train_tracks1.SM_train_tracks1"))
        (Utilities|IsValid _newestlane
          (:Is%20Valid
            (LocalVariables|Setnew%20Location (Transformation|GetWorldLocation (Variables|/Game/InfiniteMatrix/Blueprints/BP_Lane.BP_Lane_C|GetSpawnPoint _newestlane))))
          (:Is%20Not%20Valid
            _))
        (if (and (== 1 (Variables|Default|GetmeshTypeIndex)) (or (== (Variables|Default|GetmaxLanes) 1) (== (Variables|Default|GetmaxLanes) _index)))
          (LocalVariables|SetnewMesh "/Game/InfiniteMatrix/Meshes/SM_highway1.SM_highway1")
          (Development|PrintString "unmarked highway" true true "(R=0.063354,G=1.000000,B=0.152692,A=1.000000)" 5.0))
        (CallFunction|SpawnLane (LocalVariables|Getnew%20Location) (LocalVariables|GetnewMesh))))))

(fn SpawnVehicle
  (params (Spawn%20Location :type Vector))
  (Game|SpawnActorfromClass "/Game/InfiniteMatrix/Blueprints/BP_Vehicle.BP_Vehicle_C" (Math|Transform|MakeTransform Spawn%20Location "0, 0, 0" "1.000000,1.000000,1.000000") "Undefined" "MultiplyWithRoot" 0 0))